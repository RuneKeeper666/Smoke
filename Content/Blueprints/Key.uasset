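; Key collectible that exists in both the real and reflected worlds and can only be picked up in the reflected one.
; BeginPlay compares the cube's world Y to a fixed threshold, flagging real-world copies as PlayerBribed and making the player pawn their owner.
; Sphere overlap on an unflagged copy sets Collectedinator on the first-person character.
; Every key polls that shared flag on Tick and destroys itself, removing both copies together.
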(event OnComponentBeginOverlap(Sphere)
  (params (OverlappedComponent :type Primitive%20Component%20Object%20Reference) (OtherActor :type Actor%20Object%20Reference) (OtherComp :type Primitive%20Component%20Object%20Reference) (OtherBodyIndex :type Integer) (bFromSweep :type Boolean) (SweepResult :type Hit%20Result%20Structure%20%28by%20ref%29))
  ;[1 1 1] Collects item if player is in reflected world
  (bind _asbp_first_person_character (Utilities|Casting|CastToBP_FirstPersonCharacter OtherActor))
  (if (not (Variables|Default|GetPlayer%20Bribed))
    (Variables|/Game/FirstPerson/Blueprints/BP_FirstPersonCharacter.BP_FirstPersonCharacter_C|SetCollectedinator _asbp_first_person_character true)
    (Development|PrintString "Key grabinated")))

(event EventBeginPlay
  (bind _cube (Variables|Default|GetCube))
  (bind _returnvalue (Transformation|GetWorldLocation _cube))
  (bind _y (Math|Vector|BreakVector _returnvalue))
  (bind _returnvalue_2 (< _y 1.25e+03))
  ;[1 1 1] Determins if Key is in reflected world or real world
  (Variables|Default|SetPlayer%20Bribed _returnvalue_2)
  (if _returnvalue_2
    (Actor|SetOwner (Game|Player|GetPlayerPawn 0))))

(event Collision|EventActorBeginOverlap
  (params (OtherActor :type Actor%20Object%20Reference)))

(event EventTick
  (params (DeltaSeconds :type Float%20%28single-precision%29))
  ;[1 1 1] Kill's both collectebles (reflected and real) once object is reflected
  (bind _asbp_first_person_character (Utilities|Casting|CastToBP_FirstPersonCharacter (Game|Player|GetPlayerPawn 0)))
  (if (Variables|/Game/FirstPerson/Blueprints/BP_FirstPersonCharacter.BP_FirstPersonCharacter_C|GetCollectedinator _asbp_first_person_character)
    (Actor|DestroyActor)))

(fn ConstructionScript)